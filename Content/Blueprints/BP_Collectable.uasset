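; BP_Collectable is a one-time collectable pickup with casino jackpot-style feedback.
; On its first OnInteract it sets HasBeenInteracted, calls AddCollectable on the player character and plays that character's jackpot popup animation.
; It also spawns a jackpot sound and a world camera shake at its location.
; Later interactions only print a message, and the construction script adds nothing beyond the parent.
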(event `InteractableInterface.OnInteract`
  (params (Instigator :type "BaseCharacter Object Reference"))
  (bind _returnvalue (`self.K2_GetActorLocation`))
  (if (`self.bHasBeenInteracted`)
    (`KismetSystemLibrary.PrintString` "You have interacted with this!")
    (else
      (bind _asbp_player_character (cast `/Game/Blueprints/Player/BP_PlayerCharacter` (`GameplayStatics.GetPlayerCharacter` 0)))
      (set `self.bHasBeenInteracted` true)
      (`PlayerCharacter.AddCollectable` _asbp_player_character)
      (`/Game/Widgets/Popups/WBP_Popup_Jackpot.PlayPopupAnim` (`/Game/Blueprints/Player/BP_PlayerCharacter.PopupJackpotReference` _asbp_player_character))
      (`GameplayStatics.SpawnSoundAtLocation` "/Game/Sounds/Casino/CUE_Casino_Jackpot.CUE_Casino_Jackpot" _returnvalue (struct) 1.0 1.0 0.0 null null)
      (`GameplayStatics.PlayWorldCameraShake` "/Game/CameraShake/CShake_Jackpot.CShake_Jackpot_C" _returnvalue 750.0 1000.0))))

(fn `UserConstructionScript`
  (`parent.UserConstructionScript`))