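; Interactable bed actor that offers "Sleep" as its interaction text.
; Interacting opens the LV_Development_Testing level by name, with no other sleep logic.
; The hover event is empty, and BeginPlay, overlap and Tick are disabled default stubs.
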(event `InteractableInterface.OnInteract`
  (params (Instigator :type "BaseCharacter Object Reference"))
  (`GameplayStatics.OpenLevel` "LV_Development_Testing"))

(event `InteractableInterface.OnHover`
  (params (bHovered :type Boolean)))

(fn `ReturnInteractText`
  (returns (ReturnValue :type String))
  (return "Sleep"))

(fn `UserConstructionScript`
  (`parent.UserConstructionScript`))