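; Player controller for the main menu that sets up the menu camera and UI on BeginPlay.
; It views through the first CameraActor found in the level, switches input to Game and UI, and fades the camera in.
; It then creates the main menu and settings widgets, stores references to both, and adds both to the viewport up front, settings last.
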(event `self.ReceiveBeginPlay`
  (`|ExecutionSequence`
    (:`then_0`
      ; Camera Setup
      (bind _returnvalue (`GameplayStatics.GetActorOfClass` "/Script/Engine.CameraActor"))
      (`self.SetViewTargetWithBlend` _returnvalue)
      (`WidgetBlueprintLibrary.SetInputMode_GameAndUIEx` self null "DoNotLock" false)
      (`PlayerCameraManager.StartCameraFade` :`self` (`GameplayStatics.GetPlayerCameraManager` 0) :`FromAlpha` 1.0 :`Duration` 2.0))
    (:`then_1`
      ; Create Main Menu
      (bind _returnvalue_2 (`|CreateWidget` "/Game/Blueprints/Widgets/MainMenu/WBP_MainMenu.WBP_MainMenu_C" null self))
      (bind _output_get (set `self.MainMenuReference` _returnvalue_2))
      (`UserWidget.AddToViewport` _output_get 0))
    (:`then_2`
      ; Create Settings Menu
      (bind _returnvalue_3 (`|CreateWidget` "/Game/Blueprints/Widgets/MainMenu/WBP_Settings.WBP_Settings_C" null self))
      (bind _output_get_2 (set `self.SettingsMenuReference` _returnvalue_3))
      (`UserWidget.AddToViewport` _output_get_2 0))))

(fn `UserConstructionScript`)