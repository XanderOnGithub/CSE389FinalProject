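; BP_WinTrigger is an overlap trigger that ends the level with a win when the player meets the conditions.
; When BP_PlayerCharacter enters WinBox, it requires positive Money and a Collectables value equal to the number of BP_Collectable actors present at that moment.
; Success plays the Car sound and fades the camera before opening LV_Casino_Win after a delay.
; Failure only prints a lose message.
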(event `self.WinBox.OnComponentBeginOverlap`
  (params (OverlappedComponent :type "PrimitiveComponent Object Reference") (OtherActor :type "Actor Object Reference") (OtherComp :type "PrimitiveComponent Object Reference") (OtherBodyIndex :type Integer) (bFromSweep :type Boolean) (SweepResult :type "HitResult Structure (by ref)"))
  (bind _asbp_player_character (cast `/Game/Blueprints/Player/BP_PlayerCharacter` OtherActor))
  (bind _outactors (`GameplayStatics.GetAllActorsOfClass` "/Game/Blueprints/BP_Collectable.BP_Collectable_C"))
  (if (> (`PlayerCharacter.Money` _asbp_player_character) 0)
    (if (== (`PlayerCharacter.Collectables` _asbp_player_character) (`KismetArrayLibrary.Array_Length` _outactors))
      (`GameplayStatics.PlaySound2D` "/Game/Sounds/Win/Car.Car" 1.0 1.0 0.0 null null)
      (`PlayerCameraManager.StartCameraFade` :`self` (`GameplayStatics.GetPlayerCameraManager` 0) :`ToAlpha` 1.0 :`Duration` 5.0)
      (`KismetSystemLibrary.Delay` 4.9)
      (`GameplayStatics.OpenLevel` "LV_Casino_Win")
      (else
        (`KismetSystemLibrary.PrintString` "YOU LOSE" :!label _label)))
    (else
      (goto _label))))

(fn `UserConstructionScript`)