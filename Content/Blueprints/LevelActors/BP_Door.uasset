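; Double door actor that opens or closes through a SetDoorState event.
; Opening activates the NSWin and NSGlow effects, disables Frame collision and plays OpenTimeline, which lerps the R and L panels' relative transforms between their configured open transforms and identity.
; Closing restores Frame collision and runs the same timeline in reverse from its end.
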(event `SetDoorState`
  (params (`Open?` :type Boolean))
  (bind _returnvalue (`KismetMathLibrary.MakeTransform` (0.0 0.0 0.0)))
  (if `Open?`
    (`ActorComponent.Activate` (`self.NS_Win`) false)
    (`ActorComponent.Activate` (`self.NS_Glow`) false)
    (`PrimitiveComponent.SetCollisionEnabled` (`self.frame`) "NoCollision")
    (bind (_direction _alpha) (`Timeline|OpenTimeline` :!via `PlayFromStart` :!label _label)
      (:`Update`
        (`SceneComponent.K2_SetRelativeTransform` (`self.R`) (`KismetMathLibrary.TLerp` (`self.DoorROpenTransform`) _returnvalue _alpha) false false)
        (`SceneComponent.K2_SetRelativeTransform` (`self.L`) (`KismetMathLibrary.TLerp` (`self.DoorLOpenTransform`) _returnvalue _alpha) false false)))
    (else
      (`PrimitiveComponent.SetCollisionEnabled` (`self.frame`) "QueryAndPhysics")
      (goto _label :!via `ReverseFromEnd`))))

(fn `UserConstructionScript`)