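; Casino game mode that hides collectables in random slot machines and opens the door once the player has collected them all.
; InitGameMode stores the character, flags a target number of slot machines drawn at random from those in the level, and passes the total to the player HUD.
; It binds to the character's collectable and money change events; reaching the total opens the first door found, while the money handler is empty.
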(event `OnCollectablesChanged`
  (params (NewAmount :type Integer))
  (if (== NewAmount (`KismetArrayLibrary.Array_Length` (`self.Collectables`)))
    (bind _returnvalue (`GameplayStatics.GetActorOfClass` "/Game/Blueprints/LevelActors/BP_Door.BP_Door_C"))
    (`/Engine/EditorBlueprintResources/StandardMacros.IsValid` _returnvalue
      (:`Is Valid`
        (`/Game/Blueprints/LevelActors/BP_Door.SetDoorState` _returnvalue true)))))

(event `OnMoneyChanged`
  (params (NewAmount :type Integer)))

(event `InitGameMode`
  (params (Character :type "/Game/Blueprints/Player/BP_PlayerCharacter Object Reference"))
  (set `self.CharacterReference` Character)
  (`self.F_InitCollectables`)
  (set `/Game/Widgets/HUD/WBP_PlayerHUD.MaxCollectables` (`KismetArrayLibrary.Array_Length` (`self.Collectables`)) (`/Game/Blueprints/Player/BP_PlayerCharacter.PlayerHUDReference` (`self.CharacterReference`)))
  (add `PlayerCharacter.OnCollectablesChanged` (`self.CharacterReference`) (delegate `OnCollectablesChanged`))
  (add `PlayerCharacter.OnMoneyChanged` (`self.CharacterReference`) (delegate `OnMoneyChanged`)))

(fn `F_InitCollectables`
  (locals (LocalCurrentSlot :type "/Game/Blueprints/Interactables/BP_SlotMachine Object Reference"))
  (bind _localcurrentslot (`local.LocalCurrentSlot`))
  (bind _outitem (`KismetArrayLibrary.Array_Random` (`self.SlotMachines`)))
  (bind _outactors (`GameplayStatics.GetAllActorsOfClass` "/Game/Blueprints/Interactables/BP_SlotMachine.BP_SlotMachine_C"))
  (set `self.SlotMachines` _outactors)
  (for _ (range 1 (+ (`self.TargetAmountOfCollectables`) 1))
    (`/Engine/EditorBlueprintResources/StandardMacros.IsValid` _outitem
      (:`Is Valid`
        (bind _output_get (set `local.LocalCurrentSlot` _outitem))
        (`/Game/Blueprints/Interactables/BP_SlotMachine.SetCollectable` _output_get true)
        (`KismetArrayLibrary.Array_RemoveItem` (`self.SlotMachines`) _localcurrentslot)
        (`KismetArrayLibrary.Array_Add` (`self.Collectables`) _localcurrentslot)))))

(fn `UserConstructionScript`)