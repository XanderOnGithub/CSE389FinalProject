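; BP_Guard is an enemy guard character that spots the player and can be temporarily knocked into a ragdoll.
; PawnSensing flags HasSeenPlayer on the AI controller's blackboard when it sees BP_PlayerCharacter.
; DoRagdoll enables mesh physics with impact sounds and blood, ignores key capsule collisions, then after a delay moves the capsule to the mesh and restores walking.
; Destroyed only prints a debug string.
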(event `DoRagdoll`
  (params (Start :type Boolean))
  (if Start
    (if (not (`self.IsRagdolling?`))
      (`PrimitiveComponent.SetSimulatePhysics` (`self.Mesh`) true)
      (`GameplayStatics.SpawnSoundAttached` "/Game/Assets/Sounds/Push/CUE_Push_Impact.CUE_Push_Impact" (`self.Mesh`) "None" (0.0 0.0 0.0) (struct) "KeepRelativeOffset" false 1.0 1.0 0.0 null null)
      (`CharacterMovementComponent.SetMovementMode` (`self.CharacterMovement`) "MOVE_Falling" 0)
      (`PrimitiveComponent.SetCollisionResponseToChannel` (`self.CapsuleComponent`) "ECC_PhysicsBody" "ECR_Ignore")
      (`PrimitiveComponent.SetCollisionResponseToChannel` (`self.CapsuleComponent`) "ECC_Pawn" "ECR_Ignore")
      (`PrimitiveComponent.SetCollisionResponseToChannel` (`self.CapsuleComponent`) "ECC_Visibility" "ECR_Ignore")
      (`GameplayStatics.PlaySoundAtLocation` "/Game/Sounds/Voicelines/hurtgrunt.hurtgrunt" (`SceneComponent.K2_GetComponentLocation` (`self.Mesh`)) (struct) 1.0 1.0 0.0 null null null null)
      (set `self.IsRagdolling?` true)
      (`NiagaraFunctionLibrary.SpawnSystemAttached` "/Game/ParticleSystems/Pushed/NS_Blood.NS_Blood" (`self.Mesh`) "None" (0.0 0.0 0.0) (struct) "SnapToTargetIncludingScale" true)
      (`KismetSystemLibrary.Delay` 2.0)
      (`self.DoRagdoll` false))
    (elif (`self.IsRagdolling?`)
      (`SceneComponent.K2_SetWorldLocation` (`self.CapsuleComponent`) (+ (`SceneComponent.K2_GetComponentLocation` (`self.Mesh`)) (0.0 0.0 45.0)) false false)
      (`PrimitiveComponent.SetSimulatePhysics` (`self.Mesh`) false)
      (`PrimitiveComponent.SetCollisionResponseToChannel` (`self.CapsuleComponent`) "ECC_PhysicsBody" "ECR_Block")
      (`PrimitiveComponent.SetCollisionResponseToChannel` (`self.CapsuleComponent`) "ECC_Pawn" "ECR_Block")
      (`PrimitiveComponent.SetCollisionResponseToChannel` (`self.CapsuleComponent`) "ECC_Visibility" "ECR_Block")
      (set `self.IsRagdolling?` false)
      (`SceneComponent.K2_SetRelativeTransform` (`self.Mesh`) (`KismetMathLibrary.MakeTransform` (0.0 0.0 -90.0) (struct :`Yaw` -90.0)) false false)
      (`CharacterMovementComponent.SetMovementMode` (`self.CharacterMovement`) "MOVE_Walking" 0))))

(event `self.ReceiveDestroyed`
  (`KismetSystemLibrary.PrintString` "Hello"))

(event `self.PawnSensing.OnSeePawn`
  (params (Pawn :type "Pawn Object Reference"))
  (cast `/Game/Blueprints/Player/BP_PlayerCharacter` Pawn)
  (`BlackboardComponent.SetValueAsBool` (`AIBlueprintHelperLibrary.GetBlackboard` (`AIBlueprintHelperLibrary.GetAIController` self)) "HasSeenPlayer" true))

(fn `UserConstructionScript`)