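; BP_CashierDesk is an interactable cashier desk that shows a cashier popup when the player interacts with it.
; On BeginPlay it creates a WBP_Popup_Cashier with a reference to itself, assigns it to its widget component and starts it collapsed.
; Interaction makes the popup visible unless a conversation is already in progress.
; The construction script toggles the static mesh's visibility through a debug flag.
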(event `self.ReceiveBeginPlay`
  (`parent.ReceiveBeginPlay`)
  (bind _returnvalue (`|CreateWidget` "/Game/Blueprints/Widgets/Popups/WBP_Popup_Cashier.WBP_Popup_Cashier_C" null self))
  (bind _output_get (set `self.WidgetReference` _returnvalue))
  (`WidgetComponent.SetWidget` (`self.Widget`) _output_get)
  (`Widget.SetVisibility` _returnvalue "Collapsed"))

(event `self.OnInteract`
  (params (Instigator :type "BaseCharacter Object Reference"))
  (if (not (`self.bCurrentlyTalking`))
    (set `Widget.Visibility` "Visible" (`self.WidgetReference`))))

(fn `UserConstructionScript`
  (`parent.UserConstructionScript`)
  (`SceneComponent.SetVisibility` (`self.StaticMesh`) (`self.DebugVisibility`) false))