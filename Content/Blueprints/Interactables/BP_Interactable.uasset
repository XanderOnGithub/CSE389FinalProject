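; BP_Interactable is an interactable actor that responds to hover and interact events and supplies its prompt text.
; OnHover toggles custom depth rendering on its static mesh, usable for a highlight effect.
; OnInteract only prints a debug message naming the instigator and the actor, and ReturnInteractText returns the InteractText variable.
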(event `InteractableInterface.OnHover`
  (params (bHovered :type Boolean))
  (`PrimitiveComponent.SetRenderCustomDepth` (`self.StaticMesh`) bHovered))

(event `InteractableInterface.OnInteract`
  (params (Instigator :type "BaseCharacter Object Reference"))
  (`KismetSystemLibrary.PrintString` (`KismetStringLibrary.Concat_StrStr` (`KismetSystemLibrary.GetDisplayName` Instigator) " Interacted With  " (`KismetSystemLibrary.GetDisplayName` self)) true true (struct :`R` 1.0 :`B` 0.904464 :`A` 1.0) 2.0 "None"))

(fn `ReturnInteractText`
  (returns (ReturnValue :type String))
  (return (`self.InteractText`)))

(fn `UserConstructionScript`)