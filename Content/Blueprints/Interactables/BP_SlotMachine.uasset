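; Interactable slot machine that either gambles the player's money or acts as a one-time "Mythic Slot" collectable.
; Construction randomizes display and neon materials; SetCollectable overrides them with a gold and orange look, new prompt text and a spotlight.
; Normal use immediately applies a random gain or loss, then shows the money popup after a delay and re-enables itself.
; Collectable use increments the player's collectables with jackpot popup, sound, camera shake and Niagara effect.
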(event `SetCollectable`
  (params (`Collectable?` :type Boolean))
  (set `self.bIsCollectable` `Collectable?`)
  (`PrimitiveComponent.SetMaterial` (`self.StaticMesh`) 0 "/Game/Assets/Casino/Materials/Metal/MI_Gold.MI_Gold")
  (`PrimitiveComponent.SetMaterial` (`self.StaticMesh`) 2 "/Game/Assets/Casino/Materials/Slot_Machine/MI_Neon_Orange.MI_Neon_Orange")
  (set `self.InteractText` "Mythic Slot")
  (`SceneComponent.SetVisibility` (`self.SpotLight`) true false))

(event `InteractableInterface.OnInteract`
  (params (Instigator :type "BaseCharacter Object Reference"))
  (if (`self.bIsCollectable`)
    (if (not (`self.bHasBeenInteracted`))
      (bind _asbp_player_character (cast `/Game/Blueprints/Player/BP_PlayerCharacter` (`GameplayStatics.GetPlayerCharacter` 0)))
      (set `self.bHasBeenInteracted` true)
      (`PlayerCharacter.AddCollectable` _asbp_player_character)
      (`/Game/Blueprints/Widgets/Popups/WBP_Popup_Jackpot.PlayPopupAnim` (`/Game/Blueprints/Player/BP_PlayerCharacter.PopupJackpotReference` _asbp_player_character))
      (`GameplayStatics.SpawnSoundAtLocation` "/Game/Sounds/Casino/CUE_Casino_Jackpot.CUE_Casino_Jackpot" (`self.K2_GetActorLocation`) (struct) 1.0 1.0 0.0 null null)
      (`GameplayStatics.PlayWorldCameraShake` "/Game/CameraShake/CShake_Jackpot.CShake_Jackpot_C" (`self.K2_GetActorLocation`) 750.0 1000.0)
      (bind _returnvalue (`AddComponent|NODE_AddNiagaraComponent-0`))
      (`ActorComponent.Activate` _returnvalue false)
      (`SceneComponent.SetVisibility` (`self.SpotLight`) false false))
    (elif (not (`self.bHasBeenInteracted`))
      (set `self.bHasBeenInteracted` true)
      (bind _asbp_player_character_2 (cast `/Game/Blueprints/Player/BP_PlayerCharacter` (`GameplayStatics.GetPlayerCharacter` 0)))
      (bind _output_get (set `self.RandomMoney` (`KismetMathLibrary.RandomIntegerInRange` -250 500)))
      (set `PlayerCharacter.Money` (+ (`self.RandomMoney`) (`PlayerCharacter.Money` _asbp_player_character_2)) _asbp_player_character_2)
      (`GameplayStatics.SpawnSoundAtLocation` "/Game/Sounds/Casino/SlotMachine_Jägerhuus.SlotMachine_Jägerhuus" (`self.K2_GetActorLocation`) (struct) 1.0 1.0 0.0 null null)
      (bind _returnvalue_2 (`|CreateWidget` "/Game/Blueprints/Widgets/Popups/WBP_MoneyPopup.WBP_MoneyPopup_C" null _output_get))
      (`KismetSystemLibrary.Delay` 4.0)
      (`UserWidget.AddToViewport` _returnvalue_2 0)
      (set `self.bHasBeenInteracted` false))))

(fn `UserConstructionScript`
  (`parent.UserConstructionScript`)
  (`PrimitiveComponent.SetMaterial` (`self.StaticMesh`) 1 (`KismetArrayLibrary.Array_Random` (`|MakeArray` "/Game/Assets/Casino/Materials/Slot_Machine/MI_Display_1.MI_Display_1" "/Game/Assets/Casino/Materials/Slot_Machine/MI_Display_2.MI_Display_2" "/Game/Assets/Casino/Materials/Slot_Machine/MI_Display_3.MI_Display_3" :!type "MaterialInterface Object Reference")))
  (`PrimitiveComponent.SetMaterial` (`self.StaticMesh`) 2 (`KismetArrayLibrary.Array_Random` (`|MakeArray` "/Game/Assets/Casino/Materials/Slot_Machine/MI_Neon_Blue.MI_Neon_Blue" "/Game/Assets/Casino/Materials/Slot_Machine/MI_Neon_Green.MI_Neon_Green" "/Game/Assets/Casino/Materials/Slot_Machine/MI_Neon_Red.MI_Neon_Red" "/Game/Assets/Casino/Materials/Slot_Machine/MI_Neon_Violet.MI_Neon_Violet" "/Game/Assets/Casino/Materials/Slot_Machine/MI_Neon_Yellow.MI_Neon_Yellow" :!type "MaterialInterface Object Reference"))))