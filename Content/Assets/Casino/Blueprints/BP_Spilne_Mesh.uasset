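; Spline mesh Blueprint that lays a configurable mesh and material along an editable, optionally closed spline.
; The Construction Script divides the spline into equal segments, rounding up from its length over MeshLength, and adds a spline mesh component to each.
; Segment ends follow spline positions, with tangents normalized and scaled to MeshLength and a Width setting for X scale.
; It has no active runtime logic.
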(fn `UserConstructionScript`
  (bind _spline (`self.Spline`))
  (bind _width (`self.Width`))
  (bind _mesh_length (`self.Mesh Length`))
  (bind _returnvalue (`SplineComponent.GetSplineLength` (`self.Spline`)))
  (bind _returnvalue_2 (`KismetMathLibrary.FCeil` (/ _returnvalue (`self.Mesh Length`))))
  (bind _returnvalue_3 (/ _returnvalue _returnvalue_2))
  (`SplineComponent.SetClosedLoop` (`self.Spline`) (`self.Closed Loop`) true)
  (for _index (range _returnvalue_2)
    (bind _returnvalue_4 (`AddComponent|NODE_AddSplineMeshComponent-0`))
    (bind _returnvalue_5 (* _index _returnvalue_3))
    (bind _returnvalue_6 (* (+ _index 1) _returnvalue_3))
    (`SplineMeshComponent.SetStartAndEnd` _returnvalue_4 (`SplineComponent.GetLocationAtDistanceAlongSpline` _spline _returnvalue_5 "Local") (* (`KismetMathLibrary.Normal` (`SplineComponent.GetTangentAtDistanceAlongSpline` _spline _returnvalue_5 "Local")) _mesh_length) (`SplineComponent.GetLocationAtDistanceAlongSpline` _spline _returnvalue_6 "Local") (* (`KismetMathLibrary.Normal` (`SplineComponent.GetTangentAtDistanceAlongSpline` _spline _returnvalue_6 "Local")) _mesh_length) true)
    (`SplineMeshComponent.SetEndScale` _returnvalue_4 (`KismetMathLibrary.MakeVector2D` _width 1.0) true)
    (`SplineMeshComponent.SetStartScale` _returnvalue_4 (`KismetMathLibrary.MakeVector2D` _width 1.0) true)
    (`PrimitiveComponent.SetMaterial` _returnvalue_4 0 (`self.Material`))
    (`/Engine/EditorBlueprintResources/StandardMacros.IsValid` (`self.Mesh`)
      (:`Is Valid`
        (`StaticMeshComponent.SetStaticMesh` _returnvalue_4 (`self.Mesh`))))))