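; BP_Pendant_Light is a configurable casino ceiling pendant light with a wire, a fixture mesh and a spotlight.
; The construction script stretches the wire and lowers the fixture by WireLength, then applies color and emissive settings to the mesh materials.
; Shared on/off, intensity and temperature settings drive both the emissive glow and the SpotLight, which also takes an attenuation radius.
; A color temperature to RGB helper approximates blackbody color with log and power curves.
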(fn `UserConstructionScript`
  (bind _wire_length (`self.Wire Length`))
  (bind _spotlight (`self.SpotLight`))
  (`|ExecutionSequence`
    (:`then_0`
      (`SceneComponent.SetWorldScale3D` (`self.SM_Pendant_Light_Wire`) (`KismetMathLibrary.MakeVector` 1.0 1.0 (/ _wire_length 100.0)))
      (`SceneComponent.K2_SetRelativeLocation` (`self.SM_Pendant_Light`) (`KismetMathLibrary.MakeVector` 0.0 0.0 (* _wire_length -1.0)) false false)
      (`MeshComponent.SetVectorParameterValueOnMaterials` (`self.SM_Pendant_Light`) "Emissive Color" (`self.Color Temperature to RGB` (`self.Temperature`)))
      (`MeshComponent.SetVectorParameterValueOnMaterials` (`self.SM_Pendant_Light`) "Base Color" (`KismetMathLibrary.Conv_LinearColorToVector` (`KismetMathLibrary.Conv_ColorToLinearColor` (`self.Color`))))
      (`MeshComponent.SetVectorParameterValueOnMaterials` (`self.SM_Pendant_Light_Wire`) "Base Color" (`KismetMathLibrary.Conv_LinearColorToVector` (`KismetMathLibrary.Conv_ColorToLinearColor` (`self.Color`))))
      (`MeshComponent.SetScalarParameterValueOnMaterials` (`self.SM_Pendant_Light`) "Emissive Intensity" (* (`KismetMathLibrary.Conv_BoolToDouble` (`self.ON`)) (`self.Intensity (cd)`) 1.0)))
    (:`then_1`
      (`LightComponent.SetIntensity` _spotlight (`self.Intensity (cd)`))
      (`LightComponent.SetTemperature` _spotlight (`self.Temperature`))
      (`SceneComponent.SetVisibility` _spotlight (`self.ON`) false)
      (`LocalLightComponent.SetAttenuationRadius` _spotlight (`self.Attenuation Radius`)))))