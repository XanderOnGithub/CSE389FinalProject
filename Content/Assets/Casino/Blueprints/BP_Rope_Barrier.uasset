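; Casino rope barrier that builds an evenly spaced row of poles, optionally physics-simulated.
; The construction script links neighboring poles with cable components capped by end meshes when physics is on, or static meshes otherwise.
; With physics, BeginPlay re-attaches cable ends and, after a short delay, binds pole hit events.
; A hit pole checks its distance to both neighbors and releases its end of any overstretched rope.
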(event `self.ReceiveBeginPlay`
  (if (`self.Simulate Physics`)
    (for (_array_element _array_index) (`self.Ropes Array`)
      (`CableComponent.SetAttachEndToComponent` _array_element (`|GetArrayItem` (`self.Poles Array`) (+ _array_index 1)) "Rope_End1"))
    (`KismetSystemLibrary.Delay` 0.5)
    (add `PrimitiveComponent.OnComponentHit` (`self.Poles Array`) (delegate `CustomEvent`))))

(event `CustomEvent`
  (params (HitComponent :type "PrimitiveComponent Object Reference") (OtherActor :type "Actor Object Reference") (OtherComp :type "PrimitiveComponent Object Reference") (NormalImpulse :type "Vector Structure") (Hit :type "HitResult Structure (by ref)"))
  (bind _poles_array (`self.Poles Array`))
  (bind _ropes_array (`self.Ropes Array`))
  (bind _asstatic_mesh_component (cast `StaticMeshComponent` HitComponent))
  (`|ExecutionSequence`
    (:`then_0`
      (bind _returnvalue (`KismetArrayLibrary.Array_Find` _poles_array _asstatic_mesh_component))
      (bind _output (`|GetArrayItem` _poles_array (+ _returnvalue 1)))
      (`/Engine/EditorBlueprintResources/StandardMacros.IsValid` _output
        (:`Is Valid`
          (bind _returnvalue_2 (`SceneComponent.GetSocketLocation` (`|GetArrayItem` _poles_array _returnvalue) "Rope1"))
          (if (> (`KismetMathLibrary.VSize` (- (`SceneComponent.GetSocketLocation` _output "Rope1") _returnvalue_2)) 180.0)
            (bind _output_2 (`|GetArrayItem` _ropes_array _returnvalue))
            (if (and (`CableComponent.bAttachEnd` _output_2) (`CableComponent.bAttachStart` _output_2))
              (`SceneComponent.K2_DetachFromComponent` _output_2 "KeepRelative" "KeepRelative" "KeepRelative" true)
              (set `CableComponent.bAttachStart` false _output_2))))))
    (:`then_1`
      (bind _returnvalue_3 (- _returnvalue 1))
      (bind _output_3 (`|GetArrayItem` _poles_array _returnvalue_3))
      (`/Engine/EditorBlueprintResources/StandardMacros.IsValid` _output_3
        (:`Is Valid`
          (if (> (`KismetMathLibrary.VSize` (- _returnvalue_2 (`SceneComponent.GetSocketLocation` _output_3 "Rope1"))) 180.0)
            (bind _output_4 (`|GetArrayItem` _ropes_array _returnvalue_3))
            (if (and (`CableComponent.bAttachStart` _output_4) (`CableComponent.bAttachEnd` _output_4))
              (set `CableComponent.bAttachEnd` false _output_4))))))))

(fn `UserConstructionScript`
  (`|ExecutionSequence`
    (:`then_0`
      (for _index (range (`self.Poles Count`))
        (bind _returnvalue (`AddComponent|NODE_AddStaticMeshComponent-1` :`RelativeTransform` (`KismetMathLibrary.MakeTransform` (`KismetMathLibrary.MakeVector` (`KismetMathLibrary.Conv_IntToDouble` (* _index 130))))))
        (`KismetArrayLibrary.Array_Add` (`self.Poles Array`) _returnvalue)
        (`PrimitiveComponent.SetSimulatePhysics` _returnvalue (`self.Simulate Physics`))))
    (:`then_1`
      (for _index_2 (range (+ (- (`self.Poles Count`) 2) 1))
        (if (`self.Simulate Physics`)
          (bind _output (`|GetArrayItem` (`self.Poles Array`) _index_2))
          (bind _returnvalue_2 (`AddComponent|NODE_AddCableComponent-0` :`RelativeTransform` (`SceneComponent.GetSocketTransform` _output "Rope_End2" "RTS_Actor")))
          (`SceneComponent.K2_AttachToComponent` _returnvalue_2 _output "Rope_End2" "KeepWorld" "KeepWorld" "KeepRelative" false)
          (`CableComponent.SetAttachEndToComponent` _returnvalue_2 (`|GetArrayItem` (`self.Poles Array`) (+ _index_2 1)) "Rope_End1")
          (`KismetArrayLibrary.Array_Add` (`self.Ropes Array`) _returnvalue_2)
          (bind _returnvalue_3 (`AddComponent|NODE_AddStaticMeshComponent-2`))
          (`SceneComponent.K2_AttachToComponent` _returnvalue_3 _returnvalue_2 "CableEnd" "KeepRelative" "KeepRelative" "KeepRelative" true)
          (bind _returnvalue_4 (`AddComponent|NODE_AddStaticMeshComponent-3`))
          (`SceneComponent.K2_AttachToComponent` _returnvalue_4 _returnvalue_2 "CableStart" "KeepRelative" "KeepRelative" "KeepRelative" true)
          (else
            (bind _returnvalue_5 (`AddComponent|NODE_AddStaticMeshComponent-4`))
            (`SceneComponent.K2_AttachToComponent` _returnvalue_5 (`|GetArrayItem` (`self.Poles Array`) (+ _index_2 1)) "Rope1" "KeepRelative" "KeepRelative" "KeepRelative" true)))))))